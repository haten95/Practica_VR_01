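; Target spawner actor that creates either a civilian or an enemy target when SpawnEntity is called, per its comment by the Manager.
; The SpawnsCivilians flag picks the class, and the target spawns at the SpawnDirection arrow with a random sideways offset within SpreadWidth and the spawner's rotation.
; Each spawn ignores collisions and is reported through the OnEntitySpawned dispatcher, passing the new target.
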(fn ConstructionScript)

(fn SpawnEntity
  (bind _returnvalue (Transformation|GetActorRotation))
  (bind _spawndirection (Variables|Default|GetSpawnDirection))
  (bind _spreadwidth (Variables|Default|GetSpreadWidth))
  (bind _returnvalue_2 (Transformation|GetWorldLocation _spawndirection))
  (bind _returnvalue_3 (Math|Vector|GetRightVector _spawndirection))
  (bind _returnvalue_4 (* _spreadwidth -1.0))
  (bind _returnvalue_5 (Math|Random|RandomFloatinRange _returnvalue_4 _spreadwidth))
  (bind _returnvalue_6 (* _returnvalue_3 _returnvalue_5))
  (bind _returnvalue_7 (+ _returnvalue_2 _returnvalue_6))
  (bind _returnvalue_8 (Math|Transform|MakeTransform _returnvalue_7 _returnvalue))
  ;[1 1 1] SpawnEntity (lo llama el Manager): crea un civil o un enemigo segun bSpawnsCivilians, en la flecha del spawner con un desplazamiento lateral aleatorio, y avisa con OnEntitySpawned(diana).
  (if (Variables|Default|GetbSpawnsCivilians)
    (bind _returnvalue_9 (Game|SpawnActorfromClass "/Game/Blueprints/Targets/BP_Target_Civilian.BP_Target_Civilian_C" _returnvalue_8 "AlwaysSpawn" "SelectDefaultAtRuntime" 0 0))
    (Default|CallOnEntitySpawned _returnvalue_9)
    (else
      (bind _returnvalue_10 (Game|SpawnActorfromClass "/Game/Blueprints/Targets/BP_Target_Enemy.BP_Target_Enemy_C" _returnvalue_8 "AlwaysSpawn" "SelectDefaultAtRuntime" 0 0))
      (Default|CallOnEntitySpawned _returnvalue_10))))