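; BP_Target_Base is a shootable target that flies straight along its forward axis and carries a point value and time penalty.
; BeginPlay sets its ProjectileMovement velocity from MoveSpeed without Tick and gives it an eight-second lifespan.
; Weapons call OnTargetHit, which broadcasts points and time through the OnTargetDestroyed dispatcher without looking up a manager, then destroys the actor.
; A WasHit guard prevents double counting from multiple pellets.
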(event EventBeginPlay
  ;[1 1 1] Sin Tick: el ProjectileMovement (gravedad 0) mueve la entidad en linea recta hacia su eje frontal a MoveSpeed. Si nadie le dispara se autodestruye a los 8 s.
  (Actor|SetLifeSpan 8.0)
  (Game|Components|ProjectileMovement|SetVelocityinLocalSpace (Variables|Default|GetProjectileMovement) (Math|Vector|MakeVector (Variables|Default|GetMoveSpeed) 0.0 0.0)))

(fn ConstructionScript)

(fn OnTargetHit
  ;[1 1 1] OnTargetHit: la llaman las armas. Grito por el dispatcher OnTargetDestroyed(Puntos, Tiempo) y me destruyo. No busco a ningun manager. bWasHit evita contar dos veces (perdigones).
  (if (not (Variables|Default|GetbWasHit))
    (Variables|Default|SetbWasHit true)
    (Default|CallOnTargetDestroyed (Variables|Default|GetPointValue) (Variables|Default|GetTimePenalty))
    (Actor|DestroyActor)))