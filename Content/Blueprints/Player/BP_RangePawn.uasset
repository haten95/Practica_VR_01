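; VR player pawn that turns left and right shoot inputs into trigger events for held weapons.
; On possession it adds the left and right weapon Enhanced Input mapping contexts.
; Press and release actions pass through HandleTrigger, which broadcasts OnTriggerInput with the hand, pressed state and that hand's grip motion controller.
; Grabbed weapons subscribe to the dispatcher, so the pawn never calls a weapon directly.
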(event Input|EnhancedActionEvents|EnhancedInputActionIA_Shoot_Left
  (params (ActionValue :type Boolean) (ElapsedSeconds :type Float%20%28double-precision%29) (TriggeredSeconds :type Float%20%28double-precision%29) (InputAction :type Input%20Action%20Object%20Reference :default "/Game/XRFramework/Input/Actions/IA_Shoot_Left.IA_Shoot_Left"))
  (:Started
    (CallFunction|HandleTrigger true true))
  (:Completed
    (CallFunction|HandleTrigger true false)))

(event Input|EnhancedActionEvents|EnhancedInputActionIA_Shoot_Right
  (params (ActionValue :type Boolean) (ElapsedSeconds :type Float%20%28double-precision%29) (TriggeredSeconds :type Float%20%28double-precision%29) (InputAction :type Input%20Action%20Object%20Reference :default "/Game/XRFramework/Input/Actions/IA_Shoot_Right.IA_Shoot_Right"))
  (:Started
    (CallFunction|HandleTrigger false true))
  (:Completed
    (CallFunction|HandleTrigger false false)))

(event EventPossessed
  (params (NewController :type Controller%20Object%20Reference))
  (bind _returnvalue (Game|GetPlayerController 0))
  (bind _returnvalue_2 (PlayerController|LocalPlayerSubsystems|GetEnhancedInputLocalPlayerSubsystem _returnvalue))
  (Input|AddMappingContext _returnvalue_2 "/Game/XRFramework/Input/IMC_Weapon_Left.IMC_Weapon_Left" 1 "(bIgnoreAllPressedKeysUntilRelease=True,bForceImmediately=False,bNotifyUserSettings=False)")
  (Input|AddMappingContext _returnvalue_2 "/Game/XRFramework/Input/IMC_Weapon_Right.IMC_Weapon_Right" 1 "(bIgnoreAllPressedKeysUntilRelease=True,bForceImmediately=False,bNotifyUserSettings=False)"))

(fn ConstructionScript
  (|CallParentFunction))

(fn HandleTrigger
  (params (bLeft :type Boolean) (bPressed :type Boolean))
  ;[0.15 0.15 0.15 0.5] INPUT -> EVENT DISPATCHER: emite OnTriggerInput(mano izquierda?, pulsado?, mando de esa mano). Las armas cogidas se suscriben a este dispatcher; el Pawn nunca llama directamente a un arma.
  (Default|CallOnTriggerInput bLeft bPressed (select bLeft (Variables|Default|GetMotionControllerLeftGrip) (Variables|Default|GetMotionControllerRightGrip))))