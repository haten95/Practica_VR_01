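; Round-based game manager for a target-shooting game, alternating pauses and timed rounds until the final-round win or a missed score threshold.
; A one-second looping timer replaces Tick, driving the countdown, round transitions and random spawner requests.
; Chained dispatcher bindings from spawners to each spawned target feed score and time changes during rounds.
; It also spawns magazines, reloads non-pistol weapons and updates the screen widget with status and in-memory high score.
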(event EventBeginPlay
  ;[1 1 1] BEGINPLAY: busco los spawners y me suscribo a su OnEntitySpawned. Guardo las armas para rellenar arco y hacha. Empiezo en pausa (10 s) y arranco el reloj maestro (timer de 1 s, sin Tick).
  (bind _outactors (Actor|GetAllActorsOfClass "/Game/Blueprints/Targets/Spawner/BP_Target_Spawner.BP_Target_Spawner_C"))
  (bind _output_get (Variables|Default|SetAllSpawners _outactors))
  (for _array_element _output_get
    (EventDispatchers|BindEventtoOnEntitySpawned _array_element (EventDispatchers|CreateEvent :!event HandleEntitySpawned)))
  (bind _outactors_2 (Actor|GetAllActorsOfClass "/Game/Blueprints/Weapons/BP_Weapon_Base.BP_Weapon_Base_C"))
  (Variables|Default|SetAllWeapons _outactors_2)
  (Variables|Default|SetbIsRoundActive false)
  (Variables|Default|SetCurrentTime (Variables|Default|GetPauseDuration))
  (bind _returnvalue (Utilities|Time|SetTimerbyFunctionName self "MasterClockTick" 1.0 true))
  (Variables|Default|SetClockTimer _returnvalue)
  (CallFunction|UpdateScreenTexts))

(fn ConstructionScript)

(fn UpdateScreenTexts
  ;[1 1 1] UpdateScreenTexts: el propio Manager actualiza el Widget de la pantalla (SCORE x / umbral, TIME, WAVE, HIGH SCORE y estado).
  (bind _aswbp_bowling_ui (Utilities|Casting|CastToWBP_BowlingUI (UserInterface|GetUserWidgetObject (Variables|Default|GetScreen))))
  (Default|SetScore _aswbp_bowling_ui (Variables|Default|GetCurrentScore) (Variables|Default|GetThreshold) (Variables|Default|GetHighScore))
  (Default|SetTime _aswbp_bowling_ui (Variables|Default|GetCurrentTime))
  (Default|SetRound _aswbp_bowling_ui (Variables|Default|GetCurrentRound))
  (if (not (Variables|Default|GetbGameFinished))
    (Default|SetStatus _aswbp_bowling_ui (Utilities|String|SelectString "¡DISPARA!" "PAUSA - COGE MUNICION" (Variables|Default|GetbIsRoundActive)))))

(fn FinishGame
  (params (Message :type String))
  ;[1 1 1] FinishGame: paro el reloj y actualizo el High Score (solo en memoria, no se guarda al cerrar el juego).
  (Utilities|Time|ClearandInvalidateTimerbyHandle (Variables|Default|GetClockTimer))
  (Variables|Default|SetbIsRoundActive false)
  (Variables|Default|SetbGameFinished true)
  (Variables|Default|SetHighScore (Math|Integer|Max(Integer) (Variables|Default|GetHighScore) (Variables|Default|GetCurrentScore)))
  (CallFunction|UpdateScreenTexts)
  (bind _aswbp_bowling_ui (Utilities|Casting|CastToWBP_BowlingUI (UserInterface|GetUserWidgetObject (Variables|Default|GetScreen))))
  (Default|SetStatus _aswbp_bowling_ui Message))

(fn ModifyScoreandTime
  (params (PointsDelta :type Integer) (TimeDelta :type Float%20%28double-precision%29))
  ;[1 1 1] ModifyScoreAndTime: suma los puntos de la diana y los segundos de penalizacion (civil = -5 s). Solo cuenta durante la ronda.
  (if (Variables|Default|GetbIsRoundActive)
    (Variables|Default|SetCurrentScore (+ (Variables|Default|GetCurrentScore) PointsDelta))
    (Variables|Default|SetCurrentTime (Math|Integer|Max(Integer) (+ (Variables|Default|GetCurrentTime) (Math|Float|Truncate TimeDelta))))
    (CallFunction|UpdateScreenTexts)))

(fn HandleTargetDestroyed
  (params (Points :type Integer) (Time :type Float%20%28double-precision%29))
  ;[1 1 1] HandleTargetDestroyed(Points, Time): llega por el dispatcher OnTargetDestroyed de cada diana y pasa los valores a ModifyScoreAndTime.
  (CallFunction|ModifyScoreandTime Points Time))

(fn HandleEntitySpawned
  (params (Entity :type BP%20Target%20Base%20Object%20Reference))
  ;[1 1 1] Cuando un spawner crea una diana, me suscribo a SU dispatcher OnTargetDestroyed.
  (EventDispatchers|BindEventtoOnTargetDestroyed Entity (EventDispatchers|CreateEvent :!event HandleTargetDestroyed)))

(fn StartRound
  ;[1 1 1] StartRound: 45 s de ronda. Aparece 1 cargador por cada arma recargable (pistola y escopeta) y el arco y el hacha (las que no son pistola) recuperan sus 30 usos.
  (Variables|Default|SetbIsRoundActive true)
  (Variables|Default|SetCurrentTime (Variables|Default|GetRoundDuration))
  (Game|SpawnActorfromClass "/Game/Blueprints/Weapons/Ammo/BP_Magazine.BP_Magazine_C" (Variables|Default|GetMagSpotA) "AlwaysSpawn" "SelectDefaultAtRuntime" 0 0)
  (Game|SpawnActorfromClass "/Game/Blueprints/Weapons/Ammo/BP_Magazine.BP_Magazine_C" (Variables|Default|GetMagSpotB) "AlwaysSpawn" "SelectDefaultAtRuntime" 0 0)
  (for _array_element (Variables|Default|GetAllWeapons)
    (Utilities|Casting|CastToBP_Pistol _array_element
      (:CastFailed
        (Default|ReloadWeapon _array_element))))
  (CallFunction|UpdateScreenTexts))

(fn EndRound
  ;[1 1 1] EndRound: si llega al umbral y era la ronda 10 -> HAS GANADO. Si llega y no es la 10 -> ronda + 1, umbral + 500 y otra pausa de 10 s. Si no llega -> GAME OVER.
  (if (>= (Variables|Default|GetCurrentScore) (Variables|Default|GetThreshold))
    (if (>= (Variables|Default|GetCurrentRound) (Variables|Default|GetMaxRounds))
      (CallFunction|FinishGame "¡HAS GANADO!")
      (else
        (Variables|Default|SetCurrentRound (+ (Variables|Default|GetCurrentRound) 1))
        (Variables|Default|SetThreshold (+ (Variables|Default|GetThreshold) (Variables|Default|GetThresholdStep)))
        (Variables|Default|SetbIsRoundActive false)
        (Variables|Default|SetCurrentTime (Variables|Default|GetPauseDuration))
        (CallFunction|UpdateScreenTexts)))
    (else
      (CallFunction|FinishGame "GAME OVER"))))

(fn MasterClockTick
  ;[1 1 1] MasterClockTick (cada 1 s): resta un segundo. En ronda pide una entidad a un spawner al azar. Al llegar a 0: si era pausa empieza la ronda; si era ronda, EndRound.
  (Variables|Default|SetCurrentTime (- (Variables|Default|GetCurrentTime) 1))
  (CallFunction|UpdateScreenTexts)
  (if (Variables|Default|GetbIsRoundActive)
    (Default|SpawnEntity (.OutItem (Utilities|Array|Random (Variables|Default|GetAllSpawners)))))
  (if (<= (Variables|Default|GetCurrentTime) 0)
    (if (Variables|Default|GetbIsRoundActive)
      (CallFunction|EndRound)
      (else
        (CallFunction|StartRound)))))