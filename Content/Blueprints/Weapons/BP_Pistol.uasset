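; BP_Pistol is a two-handed pistol weapon that must be cocked and loaded to fire at targets.
; An overlapping BP_Magazine is destroyed to reload and clears the cocked state, which an off-hand trigger press near the slide restores.
; Firing calls the parent FireWeapon, runs a debug-drawn line trace from the muzzle that notifies BP_Target_Base hits, and plays a sound.
; Emptying the magazine clears the cocked state.
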(event OnComponentBeginOverlap(MagCollision)
  (params (OverlappedComponent :type Primitive%20Component%20Object%20Reference) (OtherActor :type Actor%20Object%20Reference) (OtherComp :type Primitive%20Component%20Object%20Reference) (OtherBodyIndex :type Integer) (bFromSweep :type Boolean) (SweepResult :type Hit%20Result%20Structure%20%28by%20ref%29))
  ;[1 1 1] RECARGA: el cargador (BP_Magazine) toca MagCollision -> se destruye, ReloadWeapon() y hay que volver a amartillar.
  (bind _asbp_magazine (Utilities|Casting|CastToBP_Magazine OtherActor))
  (Actor|DestroyActor _asbp_magazine)
  (CallFunction|ReloadWeapon)
  (Variables|Default|SetbIsCorrectlyCocked false))

(fn ConstructionScript
  (|CallParentFunction))

(fn FireWeapon
  ;[1 1 1] FireWeapon (override): solo si esta amartillada y queda municion -> Parent: FireWeapon (resta bala) -> ShootTrace -> sonido. Sin balas hay que recargar y amartillar otra vez.
  (if (and (Variables|Default|GetbIsCorrectlyCocked) (> (Variables|Default|GetCurrentAmmo) 0))
    (|CallParentFunction)
    (CallFunction|ShootTrace)
    (Audio|PlaySoundatLocation (Variables|Default|GetFireSound) (Transformation|GetWorldLocation (Variables|Default|GetMuzzleLocation)) "0, 0, 0" 1.0 1.0 0.0 0 0 0 0)
    (if (<= (Variables|Default|GetCurrentAmmo) 0)
      (Variables|Default|SetbIsCorrectlyCocked false))))

(fn OffHandTrigger
  (params (bPressed :type Boolean) (Controller :type Motion%20Controller%20Component%20Object%20Reference))
  ;[1 1 1] AMARTILLAR (override OffHandTrigger): con la otra mano en la corredera (SlideCollision, < 15 cm) y apretando su gatillo -> bIsCorrectlyCocked = true.
  (if (and bPressed (< (Math|Vector|Distance(Vector) (Transformation|GetWorldLocation (Variables|Default|GetSlideCollision)) (Transformation|GetWorldLocation Controller)) 15.0))
    (Variables|Default|SetbIsCorrectlyCocked true)))

(fn ShootTrace
  (bind _muzzlelocation (Variables|Default|GetMuzzleLocation))
  (bind _returnvalue (Transformation|GetWorldLocation _muzzlelocation))
  ;[1 1 1] ShootTrace: LineTraceByChannel desde MuzzleLocation hacia delante (TraceRange = 5000). Si toca una diana (BP_Target_Base) le llama a OnTargetHit. El rayo se dibuja 0.6 s (naranja = recorrido, rojo = impacto) para ver por donde va el disparo.
  (bind (_outhit _returnvalue_2) (Collision|LineTraceByChannel _returnvalue (+ _returnvalue (* (Math|Vector|GetForwardVector _muzzlelocation) (Variables|Default|GetTraceRange))) "TraceTypeQuery1" false 0 "ForDuration" true "(R=1.000000,G=0.550000,B=0.000000,A=1.000000)" "(R=1.000000,G=0.000000,B=0.000000,A=1.000000)" 0.6))
  (if _returnvalue_2
    (bind _asbp_target_base (Utilities|Casting|CastToBP_Target_Base (.HitActor (Collision|BreakHitResult _outhit))))
    (Default|OnTargetHit _asbp_target_base)))