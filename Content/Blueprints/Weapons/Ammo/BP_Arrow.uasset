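; BP_Arrow is an arrow projectile that registers hits on targets derived from BP_Target_Base.
; LaunchArrow marks it as launched, activates ProjectileMovement with a local forward velocity of ArrowSpeed scaled by Tension, and sets a lifespan for self-cleanup.
; Once launched, a Tip overlap with a target calls OnTargetHit and destroys the arrow, while other overlapping actors are ignored.
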(event OnComponentBeginOverlap(Tip)
  (params (OverlappedComponent :type Primitive%20Component%20Object%20Reference) (OtherActor :type Actor%20Object%20Reference) (OtherComp :type Primitive%20Component%20Object%20Reference) (OtherBodyIndex :type Integer) (bFromSweep :type Boolean) (SweepResult :type Hit%20Result%20Structure%20%28by%20ref%29))
  ;[1 1 1] La flecha lanzada toca una diana -> OnTargetHit() y la flecha se destruye.
  (if (Variables|Default|GetbLaunched)
    (bind _asbp_target_base (Utilities|Casting|CastToBP_Target_Base OtherActor))
    (Default|OnTargetHit _asbp_target_base)
    (Actor|DestroyActor)))

(fn ConstructionScript)

(fn LaunchArrow
  (params (Tension :type Float%20%28double-precision%29))
  (bind _projectilemovement (Variables|Default|GetProjectileMovement))
  ;[1 1 1] LaunchArrow(Tension): activa el ProjectileMovement con velocidad ArrowSpeed * Tension. Se autodestruye a los 6 s.
  (Variables|Default|SetbLaunched true)
  (Components|Activation|Activate _projectilemovement true)
  (Game|Components|ProjectileMovement|SetVelocityinLocalSpace _projectilemovement (Math|Vector|MakeVector (* (Variables|Default|GetArrowSpeed) Tension) 0.0 0.0))
  (Actor|SetLifeSpan 6.0))