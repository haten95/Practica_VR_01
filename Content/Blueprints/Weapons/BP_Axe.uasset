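; Throwable axe weapon that sticks into targets and returns to its starting spot on the table.
; A looping timer samples actor velocity without Tick to estimate hand speed.
; On drop, enough speed and ammo fires a shot and launches it with scaled velocity and forward spin; otherwise it simply falls.
; Hitting a BP_Target_Base while unheld freezes physics and notifies the target, and a delayed timer resets it if unheld.
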(event OnComponentHit(WeaponMesh)
  (params (HitComponent :type Primitive%20Component%20Object%20Reference) (OtherActor :type Actor%20Object%20Reference) (OtherComp :type Primitive%20Component%20Object%20Reference) (NormalImpulse :type Vector :default "0, 0, 0") (Hit :type Hit%20Result%20Structure%20%28by%20ref%29))
  ;[1 1 1] INCRUSTACION: si el hacha lanzada choca con una diana, apago las fisicas (se queda clavada) y llamo a OnTargetHit(). Si choca con otra cosa, rebota.
  (if (not (Variables|Default|GetbIsHeld))
    (bind _asbp_target_base (Utilities|Casting|CastToBP_Target_Base OtherActor))
    (Physics|SetSimulatePhysics (Variables|Default|GetWeaponMesh) false)
    (Default|OnTargetHit _asbp_target_base)))

(event EventBeginPlay
  ;[1 1 1] Guardo la posicion inicial en la mesa y arranco un temporizador (cada 0.03 s, sin Tick) que mide a que velocidad se mueve el hacha.
  (Variables|Default|SetHomeTransform (Transformation|GetActorTransform))
  (bind _returnvalue (Utilities|Time|SetTimerbyFunctionName self "TrackVelocity" 0.03 true))
  (Variables|Default|SetVelocityTimer _returnvalue))

(fn ConstructionScript
  (|CallParentFunction))

(fn ReturnHome
  (bind _weaponmesh (Variables|Default|GetWeaponMesh))
  ;[1 1 1] ReturnHome: si nadie la tiene cogida, el hacha vuelve a su sitio de la mesa.
  (if (not (Variables|Default|GetbIsHeld))
    (Physics|SetSimulatePhysics _weaponmesh false)
    (Transformation|SetActorTransform (Variables|Default|GetHomeTransform) false true)
    (Physics|SetSimulatePhysics _weaponmesh true)))

(fn OnWeaponDropped
  (bind _handvelocity (Variables|Default|GetHandVelocity))
  (bind _weaponmesh (Variables|Default|GetWeaponMesh))
  ;[1 1 1] LANZAR o SOLTAR (override OnWeaponDropped): uso la velocidad medida por TrackVelocity justo antes de soltar. Si supera ThrowMinSpeed (150 cm/s) es un lanzamiento: gasta 1, fisicas on, sale con esa velocidad x ThrowMultiplier y girando hacia delante (SpinSpeed). Si va mas lento solo la dejo caer. En los dos casos vuelve a la mesa a los ReturnDelay segundos.
  (if (and (> (Math|Vector|VectorLength _handvelocity) (Variables|Default|GetThrowMinSpeed)) (> (Variables|Default|GetCurrentAmmo) 0))
    (CallFunction|FireWeapon)
    (|CallParentFunction)
    (Physics|SetSimulatePhysics _weaponmesh true)
    (Class|PrimitiveComponent|SetNotifyRigidBodyCollision _weaponmesh true)
    (Physics|SetPhysicsLinearVelocity _weaponmesh (* _handvelocity (Variables|Default|GetThrowMultiplier)) false "None")
    (Class|PrimitiveComponent|SetPhysicsAngularVelocityinDegrees _weaponmesh (* (Math|Vector|CrossProduct "0.000000,0.000000,1.000000" (Math|Vector|Normalize _handvelocity)) (Variables|Default|GetSpinSpeed)) false "None")
    (else
      (|CallParentFunction)
      (Physics|SetSimulatePhysics (Variables|Default|GetWeaponMesh) true)))
  (bind _returnvalue (Utilities|Time|SetTimerbyFunctionName self "ReturnHome" (Variables|Default|GetReturnDelay)))
  (Variables|Default|SetReturnTimer _returnvalue))

(fn TrackVelocity
  (bind _returnvalue (Transformation|GetActorLocation))
  ;[1 1 1] TrackVelocity: velocidad = (posicion ahora - posicion anterior) / 0.03 s. Mientras la llevo en la mano es la velocidad de mi mano.
  (Variables|Default|SetHandVelocity (* (- _returnvalue (Variables|Default|GetLastLocation)) 33.333))
  (Variables|Default|SetLastLocation _returnvalue))