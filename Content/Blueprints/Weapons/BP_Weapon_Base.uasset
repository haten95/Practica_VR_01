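; Base VR weapon that child weapons extend with their own firing behavior, such as traces, arrows or throws.
; Grabbing stores the holding motion controller and binds to BP_RangePawn's OnTriggerInput dispatcher, avoiding Tick; dropping unbinds.
; The holding hand's trigger calls FireWeapon or StopFireWeapon, while the other hand's goes to the empty OffHandTrigger hook.
; FireWeapon spends one round only while held with ammo left, and ReloadWeapon refills to MaxAmmo.
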(event OnGrabbed(GrabComponent)
  ;[1 1 1] AL COGER: guardo el mando que me sujeta y me suscribo al dispatcher OnTriggerInput del pawn (sin Tick).
  (bind _output_get (Variables|Default|SetHoldingController (Variables|/Game/XRFramework/Blueprints/BP_GrabComponent.BP_GrabComponent_C|GetMotionControllerRef (Variables|Default|GetGrabComponent))))
  (bind _asbp_range_pawn (Utilities|Casting|CastToBP_RangePawn (Components|GetOwner _output_get))
    (:then
      (bind _output_get_2 (Variables|Default|SetInputSource _asbp_range_pawn))
      (EventDispatchers|BindEventtoOnTriggerInput _output_get_2 (EventDispatchers|CreateEvent :!event HandleTriggerInput))
      (CallFunction|OnWeaponGrabbed))
    (:CastFailed
      (CallFunction|OnWeaponGrabbed))))

(event OnDropped(GrabComponent)
  (bind _inputsource (Variables|Default|GetInputSource))
  ;[1 1 1] AL SOLTAR: me desuscribo del pawn y aviso a OnWeaponDropped (el hacha lo usa para lanzarse).
  (Utilities|IsValid _inputsource
    (:Is%20Valid
      (EventDispatchers|UnbindEventfromOnTriggerInput _inputsource (EventDispatchers|CreateEvent :!event HandleTriggerInput)))
    (:Is%20Not%20Valid
      _))
  (CallFunction|OnWeaponDropped))

(fn ConstructionScript)

(fn FireWeapon
  ;[1 1 1] FireWeapon (padre): solo dispara si el arma esta cogida y le queda municion. Resta 1 bala. Las hijas hacen el resto (trazo, flecha, lanzamiento).
  (if (and (Variables|Default|GetbIsHeld) (> (Variables|Default|GetCurrentAmmo) 0))
    (Variables|Default|SetCurrentAmmo (- (Variables|Default|GetCurrentAmmo) 1))))

(fn StopFireWeapon)

(fn ReloadWeapon
  ;[1 1 1] ReloadWeapon: CurrentAmmo = MaxAmmo
  (Variables|Default|SetCurrentAmmo (Variables|Default|GetMaxAmmo)))

(fn OnWeaponGrabbed
  (Variables|Default|SetbIsHeld true))

(fn OnWeaponDropped
  (Variables|Default|SetbIsHeld false))

(fn OffHandTrigger
  (params (bPressed :type Boolean) (Controller :type Motion%20Controller%20Component%20Object%20Reference)))

(fn HandleTriggerInput
  (params (bLeftHand :type Boolean) (bPressed :type Boolean) (Controller :type Motion%20Controller%20Component%20Object%20Reference))
  ;[1 1 1] Se llama por el dispatcher OnTriggerInput del pawn. Mano que sujeta: gatillo = FireWeapon / soltar = StopFireWeapon. La otra mano: OffHandTrigger (amartillar, tensar).
  (if (== Controller (Variables|Default|GetHoldingController))
    (if bPressed
      (CallFunction|FireWeapon)
      (else
        (CallFunction|StopFireWeapon)))
    (else
      (CallFunction|OffHandTrigger bPressed Controller))))