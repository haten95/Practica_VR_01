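; BP_Shotgun is a shotgun weapon derived from BP_Pistol that keeps the parent's reload and cocking and overrides only the shot trace.
; ShootTrace fires PelletCount Visibility line traces from MuzzleLocation, each randomized within a SpreadAngle cone and reaching TraceRange, with timed debug drawing.
; Each pellet that hits a BP_Target_Base calls OnTargetHit on it, so one shot can trigger a target several times.
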(fn ConstructionScript
  (|CallParentFunction))

(fn ShootTrace
  (bind _muzzlelocation (Variables|Default|GetMuzzleLocation))
  (bind _returnvalue (Transformation|GetWorldLocation _muzzlelocation))
  ;[1 1 1] ESCOPETA (hija de BP_Pistol): misma recarga y amartillado; solo cambia ShootTrace: PelletCount perdigones con dispersion SpreadAngle. Cada disparo gasta 1 cartucho.
  (for _index (range 0 (- (Variables|Default|GetPelletCount) 1))
    (bind (_outhit _returnvalue_2) (Collision|LineTraceByChannel _returnvalue (+ _returnvalue (* (Math|Random|RandomUnitVectorinConeinDegrees (Math|Vector|GetForwardVector _muzzlelocation) (Variables|Default|GetSpreadAngle)) (Variables|Default|GetTraceRange))) "TraceTypeQuery1" false 0 "ForDuration" true "(R=1.000000,G=0.550000,B=0.000000,A=1.000000)" "(R=1.000000,G=0.000000,B=0.000000,A=1.000000)" 0.6))
    (if _returnvalue_2
      (bind _asbp_target_base (Utilities|Casting|CastToBP_Target_Base (.HitActor (Collision|BreakHitResult _outhit))))
      (Default|OnTargetHit _asbp_target_base))))