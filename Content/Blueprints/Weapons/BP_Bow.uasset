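; VR-style bow weapon, a child of BP_Weapon_Base, that the off hand draws and releases to shoot arrows.
; Pressing the off-hand trigger near StringCollision, with ammo left, spawns a BP_Arrow attached to the muzzle and records the pulling hand.
; Releasing that trigger calls StopFireWeapon, which runs FireWeapon to spend ammo, detaches the arrow and launches it with tension from the clamped hand-to-muzzle distance.
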(event EventBeginPlay
  (|CallParentFunction) ; This node is disabled and will not be called.\nDrag off pins to build functionality.
)

(event Collision|EventActorBeginOverlap
  (params (OtherActor :type Actor%20Object%20Reference))
  ;[1 1 1] ARCO (hijo de BP_Weapon_Base): toda la logica esta en los overrides OffHandTrigger (tensar con la otra mano) y StopFireWeapon (soltar el gatillo = disparar).
  (|CallParentFunction OtherActor) ; This node is disabled and will not be called.\nDrag off pins to build functionality.
)

(fn ConstructionScript
  (|CallParentFunction))

(fn OffHandTrigger
  (params (bPressed :type Boolean) (Controller :type Motion%20Controller%20Component%20Object%20Reference))
  (bind _muzzlelocation (Variables|Default|GetMuzzleLocation))
  ;[1 1 1] TENSAR: la otra mano aprieta el gatillo junto a la cuerda (StringCollision) -> aparece una BP_Arrow acoplada al arco y guardo la mano que tira.
  (if bPressed
    (if (and (and (< (Math|Vector|Distance(Vector) (Transformation|GetWorldLocation (Variables|Default|GetStringCollision)) (Transformation|GetWorldLocation Controller)) (Variables|Default|GetStringReach)) (not (Utilities|IsValid (Variables|Default|GetSpawnedArrow)))) (> (Variables|Default|GetCurrentAmmo) 0))
      (bind _returnvalue (Game|SpawnActorfromClass "/Game/Blueprints/Weapons/Ammo/BP_Arrow.BP_Arrow_C" (Transformation|GetWorldTransform _muzzlelocation) "AlwaysSpawn" "SelectDefaultAtRuntime" 0 0))
      (bind _output_get (Variables|Default|SetSpawnedArrow _returnvalue))
      (Transformation|AttachComponentToComponent _output_get _muzzlelocation "None" "SnapToTarget" "SnapToTarget" "KeepWorld" true)
      (Variables|Default|SetPullingHand Controller))
    (else
      ;[1 1 1] SOLTAR EL GATILLO de la mano que tira -> StopFireWeapon (dispara la flecha).
      (if (and (Utilities|IsValid (Variables|Default|GetSpawnedArrow)) (== (Variables|Default|GetPullingHand) Controller))
        (CallFunction|StopFireWeapon)))))

(fn StopFireWeapon
  ;[1 1 1] StopFireWeapon (override): FireWeapon() gasta 1 flecha; tension = distancia mano-arco / 50, limitada entre 0.2 y 1.0; se desacopla la flecha y LaunchArrow(tension). Limpio SpawnedArrow y PullingHand.
  (if (Utilities|IsValid (Variables|Default|GetSpawnedArrow))
    (CallFunction|FireWeapon)
    (Transformation|DetachFromActor (Variables|Default|GetSpawnedArrow) "KeepWorld" "KeepWorld" "KeepWorld")
    (Default|LaunchArrow (Variables|Default|GetSpawnedArrow) (Math|Float|Clamp(Float) (/ (Math|Vector|Distance(Vector) (Transformation|GetWorldLocation (Variables|Default|GetPullingHand)) (Transformation|GetWorldLocation (Variables|Default|GetMuzzleLocation))) 5e+01) 0.2))
    (Variables|Default|SetSpawnedArrow 0)
    (Variables|Default|SetPullingHand 0)))